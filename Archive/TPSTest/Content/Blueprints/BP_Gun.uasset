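; BP_Gun is a weapon that spawns BP_Projectile at its muzzle arrow and counts down limited ammo.
; Single shots pass through a DoOnce reset after a delay, while rapid fire runs a looping timer on Fire that ReleaseTrigger clears.
; The owner pawn supplies ammo and fire delay through InitialiseWeaponStats, whose RapidFire flag selects which delay variable is set.
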(event Custom|PullTriggerOnce
  (Utilities|FlowControl|DoOnce false :!label _label
    (:Completed
      (Variables|Default|SetbFiring true)
      (CallFunction|Fire)
      (Utilities|FlowControl|Delay (Variables|Default|GetFireDelay))
      (goto _label Reset))))

(fn ConstructionScript)

(fn Fire
  (bind _muzzlearrowcomp (Variables|Default|GetMuzzleArrowComp))
  ;[1 1 1] Spawn Projectile at MuzzleArrowComp.
  (if (>= (Variables|Default|GetLimitAmmo) 0)
    (if (Variables|Default|GetbFiring)
      (Game|SpawnActorfromClass "/Game/Projectile/BP_Projectile.BP_Projectile_C" (Math|Transform|MakeTransform (Transformation|GetWorldLocation _muzzlearrowcomp) (Transformation|GetWorldRotation _muzzlearrowcomp)) "Undefined" 0 self)
      (Transformation|AttachComponentToComponent (Variables|Default|GetMuzzleArrowComp) 0 "None" "KeepWorld" "KeepWorld" "KeepWorld" true)
      (Math|Integer|DecrementInt (Variables|Default|GetLimitAmmo)))))

(fn PullTriggerRapidFire
  ;[1 1 1] Bind to Press Input
  (Utilities|FlowControl|Sequence
    (:then_0
      (Variables|Default|SetbFiring true)
      (CallFunction|Fire))
    (:then_1
      (Utilities|Time|SetTimerbyFunctionName self "Fire" (Variables|Default|GetRapidFireDelay) true))))

(fn ReleaseTrigger
  ;[1 1 1] Bind to Release Input
  (Utilities|Time|ClearTimerbyFunctionName self "Fire"))

(fn InitialiseWeaponStats
  (params (DelayFire :type Float%20%28single-precision%29) (LimitAmmo :type Integer) (bRapidFire :type Boolean))
  ;[1 1 1] Sets Weapon Stats , Call in Owner Pawn
  (Utilities|FlowControl|Sequence
    (:then_0
      ;[1 1 1] Delay Between Firing
      (if bRapidFire
        ;;[1 1 1] With Rapid Fire
        (Variables|Default|SetRapidFireDelay DelayFire)
        (else
          ;;[1 1 1] Without RapidFire
          (Variables|Default|SetFireDelay DelayFire))))
    (:then_1
      (Variables|Default|SetLimitAmmo LimitAmmo))))