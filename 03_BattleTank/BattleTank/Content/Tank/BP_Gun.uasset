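; BP_Gun is a rapid-fire weapon in the Tank folder that spawns and launches BP_Projectile while its trigger is held.
; PullTrigger sets Firing, shoots immediately and starts a looping Fire timer at RapidFireDelay, which ReleaseTrigger clears.
; Fire spawns each projectile at the Arrow component's transform, launches it and decrements LimitAmmo.
; The ammo check accepts zero, so one shot still fires when LimitAmmo is 0.
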(event Collision|EventActorBeginOverlap
  (params (OtherActor :type Actor%20Object%20Reference)))

(fn ConstructionScript)

(fn Fire
  (bind _arrow (Variables|Default|GetArrow))
  (if (>= (Variables|Default|GetLimitAmmo) 0)
    (if (Variables|Default|GetbFiring)
      (bind _returnvalue (Game|SpawnActorfromClass "/Game/Projectile/BP_Projectile.BP_Projectile_C" (Math|Transform|MakeTransform (Transformation|GetWorldLocation _arrow) (Transformation|GetWorldRotation _arrow)) "Undefined" 0 self))
      (Class|Projectile|LaunchProjectile _returnvalue 2e+04)
      (Math|Integer|DecrementInt (Variables|Default|GetLimitAmmo)))))

(fn PullTrigger
  (Variables|Default|SetbFiring true)
  (CallFunction|Fire)
  (Utilities|Time|SetTimerbyFunctionName self "Fire" (Variables|Default|GetRapidFireDelay) true))

(fn ReleaseTrigger
  (Utilities|Time|ClearTimerbyFunctionName self "Fire")
  (Variables|Default|SetbFiring false))